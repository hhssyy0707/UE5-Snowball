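; BP_NPC is an enemy that rolls a snowball toward the player and launches it at close range.
; A Tick-driven Idle/Move/Attack state machine spawns and attaches a BP_Snowball, chases the player while spinning it, then switches to Attack within range.
; Attack detaches the ball and translates it along the NPC's forward vector, without physics.
; Impact explosion and return to Idle are disconnected, so Attack never exits.
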(event EventBeginPlay)

(event Collision|EventActorBeginOverlap
  (params (OtherActor :type Actor%20Object%20Reference)))

(event EventTick
  (params (DeltaSeconds :type Float%20%28single-precision%29))
  (switch Utilities|FlowControl|Switch|SwitchonBP_EEnemyState (Variables|Default|GetEnemyState)
    (:NewEnumerator0
      (bind _output_get (Variables|Default|SetEnemy (Game|Player|GetPlayerPawn 0)))
      (Utilities|IsValid _output_get
        (:Is%20Valid
          (Variables|Default|GetSnowball
            (:then)
            (:else
              (CallFunction|Idle (Variables|Default|GetEnemy))
              (Variables|Default|SetEnemyState "NewEnumerator1"))))))
    (:NewEnumerator1
      (CallFunction|LookatTarget)
      (CallFunction|BallRotation (Variables|Default|GetEnemySpeed))
      (CallFunction|Move (Variables|Default|GetEnemy))
      (if (< (Math|Vector|Distance(Vector) (Transformation|GetActorLocation (Variables|Default|GetEnemy)) (Transformation|GetActorLocation self)) 7e+02)
        (Variables|Default|SetEnemyState "NewEnumerator3")))
    (:NewEnumerator3
      (CallFunction|Attack))))

(fn ConstructionScript)

(fn Translate
  (params (Speed :type Float%20%28double-precision%29) (Direction :type Vector) (TargetMoved :type Actor%20Object%20Reference))
  (Utilities|IsValid TargetMoved
    (:Is%20Valid
      (Transformation|SetActorLocation TargetMoved (+ (Transformation|GetActorLocation TargetMoved) (* Speed (Math|Vector|Normalize Direction) (Utilities|Time|GetWorldDeltaSeconds))) false false))))

(fn Move
  (params (TargetObject :type Actor%20Object%20Reference))
  (CallFunction|Translate (Variables|Default|GetEnemySpeed) (- (Transformation|GetActorLocation TargetObject) (Transformation|GetActorLocation)) self))

(fn BallRotation
  (params (Speed :type Float%20%28double-precision%29))
  (bind _snowball (Variables|Default|GetSnowball)
    (:then
      (Transformation|AddLocalRotation (Variables|/Game/MyBluePrint/BP_Snowball.BP_Snowball_C|GetSnowball _snowball) (Math|Rotator|MakeRotator 0.0 (* Speed (Utilities|Time|GetWorldDeltaSeconds) -1.0) 0.0) false false))
    (:else)))

(fn LookatTarget
  (bind _enemy (Variables|Default|GetEnemy)
    (:then
      (Transformation|SetActorRotation (Math|Rotator|FindLookatRotation (Transformation|GetActorLocation) (Transformation|GetActorLocation _enemy))))
    (:else)))

(fn Idle
  (params (Enemy :type Actor%20Object%20Reference))
  (Variables|Default|SetEnemy Enemy)
  (bind _returnvalue (Game|SpawnActorfromClass "/Game/MyBluePrint/BP_Snowball.BP_Snowball_C" (Math|Transform|MakeTransform "0, 0, 0" "0, 0, 0" "1.000000,1.000000,1.000000") "Undefined" "MultiplyWithRoot" self 0))
  (bind _output_get (Variables|Default|SetSnowball _returnvalue))
  (Transformation|AttachComponentToComponent _output_get (Variables|Collision|GetCapsuleComponent) "None" "SnapToTarget" "SnapToTarget" "SnapToTarget" true)
  (Transformation|SetActorRelativeLocation (Variables|Default|GetSnowball) "100.000000,0.000000,1.000000"))

(fn Attack
  (bind _snowball (Variables|Default|GetSnowball)
    (:then
      (Transformation|DetachFromActor _snowball "KeepWorld" "KeepWorld" "KeepWorld")
      (CallFunction|ThrowBall)
      (CallFunction|BallRotation (Variables|Default|GetSnowballSpeed)))
    (:else)))

(fn NewFunction)

(fn ThrowBall
  (bind _snowball (Variables|Default|GetSnowball)
    (:then
      (CallFunction|Translate (Variables|Default|GetEnemySpeed) (Transformation|GetActorForwardVector) _snowball))
    (:else)))